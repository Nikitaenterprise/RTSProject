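; Gameplay Ability that sends a ship to gather resources from the closest asteroid field.
; On activation, a GoToClosestResource task runs, and on arrival the ability fetches that field's asteroids and their count.
; A GatherResource task works through the asteroids by index, looping to the next whenever one is consumed.
; The ability ends when cargo is full or the last asteroid is consumed.
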(event Ability|EventActivateAbility
  (bind _closestasteroidfield (|GotoClosestResource 0.0)
    (:OnDestinationReached
      (bind _returnvalue (Class|AsteroidField|GetNumberOfAsteroidsinField _closestasteroidfield))
      (Variables|Default|SetNumberOfAsteroids _returnvalue)
      (bind _returnvalue_2 (Class|AsteroidField|GetAsteroids _closestasteroidfield))
      (|GatherResource (Utilities|Array|Get(acopy) _returnvalue_2 (Variables|Default|GetCurrentAsteroidNumber)) :!label _label
        (:OnCargoFull
          (Ability|EndAbility))
        (:OnResourceConsumed
          (if (< (+ (Variables|Default|GetCurrentAsteroidNumber) 1) (Variables|Default|GetNumberOfAsteroids))
            (Variables|Default|SetCurrentAsteroidNumber (+ (Variables|Default|GetCurrentAsteroidNumber) 1))
            (goto _label)
            (else
              (Ability|EndAbility))))))))

(event Ability|EventOnEndAbility
  (params (bWasCancelled :type Boolean)))