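; Gameplay ability that sends a worker ship to gather from the resource closest to it, looked up through the RTS game mode's resource manager.
; A TransferResource task moves resources into the worker, while WaitForOrderChange ends that task and the ability when orders change.
; Full cargo or a consumed resource applies GE_HasSomeCargo to the owner and ends the ability, as does a missing manager, without the effect.
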(event Ability|EventActivateAbility
  (bind _returnvalue (Ability|GetOwningActorfromActorInfo))
  (bind _returnvalue_2 (Class|RTSGameMode|GetRTSGameMode))
  (bind _returnvalue_3 (Class|RTSGameMode|GetResourceManager _returnvalue_2))
  (Ability|CommitAbility)
  (Utilities|IsValid _returnvalue_2
    (:Is%20Valid
      (Utilities|IsValid _returnvalue_3
        (:Is%20Valid
          (bind _returnvalue_4 (Class|ResourceManager|GetClosestResource _returnvalue_3 (Transformation|GetActorLocation _returnvalue)))
          (bind _asynctaskproxy (|TransferResource _returnvalue _returnvalue_4)
            (:then
              (|WaitforOrderChange 0 (Utilities|Array|MakeArray _asynctaskproxy)
                (:OnOrderChanged
                  _)))
            (:OnCargoFull
              (Ability|ApplyGameplayEffectToOwner "/Game/Actors/Ship/Worker/GameplayEffects/GE_HasSomeCargo.GE_HasSomeCargo_C" :!label _label))
            (:OnResourceConsumed
              (goto _label)))
          (Ability|EndAbility))
        (:Is%20Not%20Valid
          (Ability|EndAbility :!label _label_2))))
    (:Is%20Not%20Valid
      (goto _label_2))))