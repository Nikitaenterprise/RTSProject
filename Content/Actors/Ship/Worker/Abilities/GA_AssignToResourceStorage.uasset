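; Gameplay ability that lets the player assign a resource storage building to a Worker by clicking it.
; On activation it commits, switches the HUD cursor to the gather-resource cursor and starts a WaitForMouseClick task.
; A left click traces under the cursor; a ResourceStorage building becomes the worker's container and ends the ability, while other buildings only print debug text.
; Ending the ability stops the task and restores the default cursor.
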(event Ability|EventActivateAbility
  (bind _returnvalue (Class|GameplayStatics|GetPlayerControllerfromID))
  (bind _asworker (Utilities|Casting|CastToWorker (Ability|GetOwningActorfromActorInfo)))
  (Ability|CommitAbility)
  (Utilities|IsValid _returnvalue
    (:Is%20Valid
      (bind _asgame_hud (Utilities|Casting|CastToGameHUD (HUD|GetHUD _returnvalue))
        (:then
          (Utilities|IsValid (Class|GameHUD|GetMouseCursorWidget _asgame_hud)
            (:Is%20Valid
              (Class|MouseCursorWidget|SetCursorfromAbility (Class|GameHUD|GetMouseCursorWidget _asgame_hud) "/Game/Actors/Ship/Worker/Abilities/GatherResourceCursor.GatherResourceCursor"))
            (:Is%20Not%20Valid
              _)))
        (:CastFailed
          _)))
    (:Is%20Not%20Valid
      _))
  (bind _asynctaskproxy (|WaitforMouseClick)
    (:then
      (Variables|Default|SetAsync%20Task _asynctaskproxy))
    (:OnLMBClicked
      (bind _asbuilding (Utilities|Casting|CastToBuilding (.hitactor (.HitResult (Game|Player|GetHitResultUnderCursorbyChannel (Game|GetPlayerController 0) "TraceTypeQuery1" true)))))
      (if (Utilities|Enum|Equal(Enum) (Class|Building|GetBuildingType _asbuilding) "ResourceStorage")
        (Class|Worker|SetResourceContainerBuilding _asworker _asbuilding)
        (Ability|EndAbility)
        (else
          (Development|PrintString "Hello"))))))

(event Ability|EventOnEndAbility
  (params (bWasCancelled :type Boolean))
  (bind _returnvalue (Class|GameplayStatics|GetPlayerControllerfromID))
  (GameplayTasks|EndTask (Variables|Default|GetAsync%20Task))
  (Utilities|IsValid _returnvalue
    (:Is%20Valid
      (bind _asgame_hud (Utilities|Casting|CastToGameHUD (HUD|GetHUD _returnvalue)))
      (Utilities|IsValid (Class|GameHUD|GetMouseCursorWidget _asgame_hud)
        (:Is%20Valid
          (Class|MouseCursorWidget|SetCursortoDefault (Class|GameHUD|GetMouseCursorWidget _asgame_hud)))))))