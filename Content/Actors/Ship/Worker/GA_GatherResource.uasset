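; Gameplay ability for worker ships that travels to the closest asteroid field and gathers resources from it.
; An ability task moves the ship there; on arrival the ability commits and runs GatherResource on each asteroid in turn, advancing when one is consumed.
; When cargo is full or the asteroids run out, it applies GE_HasSomeCargo and ends.
; If no adjacent resource is found, it ends without committing.
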(event Ability|EventActivateAbility
  (bind _closestasteroidfield (|GotoClosestResource 5e+02)
    (:OnDestinationReached
      (bind _returnvalue (Class|AsteroidField|GetNumberOfAsteroidsinField _closestasteroidfield))
      (Variables|Default|SetNumberOfAsteroids _returnvalue)
      (bind _returnvalue_2 (Class|AsteroidField|GetAsteroids _closestasteroidfield))
      (Ability|CommitAbility)
      (|GatherResource (Utilities|Array|Get(acopy) _returnvalue_2 (Variables|Default|GetCurrentAsteroidNumber)) :!label _label
        (:OnCargoFull
          _)
        (:OnResourceConsumed
          (if (< (+ (Variables|Default|GetCurrentAsteroidNumber) 1) (Variables|Default|GetNumberOfAsteroids))
            (Variables|Default|SetCurrentAsteroidNumber (+ (Variables|Default|GetCurrentAsteroidNumber) 1))
            (goto _label)
            (else
              _))))
      (Ability|ApplyGameplayEffectToOwner "/Game/Actors/Ship/Worker/GE_HasSomeCargo.GE_HasSomeCargo_C")
      (Ability|EndAbility))
    (:NoAdjacentResourceFound
      (Ability|EndAbility))))