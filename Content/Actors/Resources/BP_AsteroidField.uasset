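; Asteroid field resource actor that scatters randomly sized asteroids and reports a resource amount from their scale.
; The construction script adds a random number of instanced static meshes with random rotation and uniform scale.
; Positions multiply the box extent by random unit vectors, placing asteroids on an ellipsoid shell rather than throughout the volume.
; GetResourceAmount overwrites its total each loop, so it returns only the last iteration's scale length times a constant.
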(fn ConstructionScript
  (bind _box (Variables|Default|GetBox))
  (bind _output_get (Variables|Default|SetNumberOfAsteroids (Math|Random|RandomIntegerinRange 10 30)))
  (for _index (range 0 _output_get)
    (Components|InstancedStaticMesh|AddInstance (Variables|Default|GetInstancedStaticMesh) (Math|Transform|MakeTransform (+ (* (Components|Box|GetScaledBoxExtent _box) (Math|Random|RandomUnitVector)) (Variables|/Script/Engine.SceneComponent|GetRelativeLocation _box)) (Math|Random|RandomRotator false) (Math|Conversions|ToVector(Float) (Math|Random|RandomFloatinRange 0.2 1.0))))))

(fn GetResourceAmount
  (bind _instancedstaticmesh (Variables|Default|GetInstancedStaticMesh))
  (for _index (range 0 (Components|InstancedStaticMesh|GetInstanceCount _instancedstaticmesh))
    (LocalVariables|SetTotal%20scale (Math|Vector|VectorLength (.scale (.OutInstanceTransform (Components|InstancedStaticMesh|GetInstanceTransform _instancedstaticmesh _index true))))))
  (return (* (LocalVariables|GetTotal%20scale) 1e+04)))