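; BP_PlayerAIController is the AI controller for a player, driving its possessed pawn through a behavior tree.
; On possess it sets up the BB_Player blackboard and runs BT_PlayerMain, leaving the decisions to that tree.
; An unconnected chain, which never runs, would spawn a blue ship after a delay and order it to move via its ship AI controller's blackboard.
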(event EventBeginPlay)

(event EventPossess
  (params (PossessedPawn :type Pawn%20Object%20Reference))
  (Class|AIController|UseBlackboard "/Game/Actors/Player/BB_Player.BB_Player")
  (AI|RunBehaviorTree "/Game/Actors/Player/BT_PlayerMain.BT_PlayerMain"))

(fn ConstructionScript)